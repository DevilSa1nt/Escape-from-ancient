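; Two-way teleporter Blueprint that moves a BP_TopDownCharacter between its Start and End components.
; Overlapping either component teleports the character to the other's world location without sweeping.
; A shared IsTp flag with a one-second delay blocks immediate bounce-back.
; The construction script offsets and scales both components from location and scale variables, allowing placement to be set per instance.
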(event `self.Start.OnComponentBeginOverlap`
  (params (OverlappedComponent :type "PrimitiveComponent Object Reference") (OtherActor :type "Actor Object Reference") (OtherComp :type "PrimitiveComponent Object Reference") (OtherBodyIndex :type Integer) (bFromSweep :type Boolean) (SweepResult :type "HitResult Structure (by ref)"))
  (if (not (`self.bIsTp`))
    (bind _asbp_top_down_character (cast `/Game/TopDown/Blueprints/BP_TopDownCharacter` OtherActor))
    (set `self.bIsTp` true)
    (`self.K2_SetActorLocation` _asbp_top_down_character (`SceneComponent.K2_GetComponentLocation` (`self.End`)) false true)
    (`KismetSystemLibrary.Delay` 1.0)
    (set `self.bIsTp` false)))

(event `self.End.OnComponentBeginOverlap`
  (params (OverlappedComponent :type "PrimitiveComponent Object Reference") (OtherActor :type "Actor Object Reference") (OtherComp :type "PrimitiveComponent Object Reference") (OtherBodyIndex :type Integer) (bFromSweep :type Boolean) (SweepResult :type "HitResult Structure (by ref)"))
  (if (not (`self.bIsTp`))
    (bind _asbp_top_down_character (cast `/Game/TopDown/Blueprints/BP_TopDownCharacter` OtherActor))
    (set `self.bIsTp` true)
    (`self.K2_SetActorLocation` _asbp_top_down_character (`SceneComponent.K2_GetComponentLocation` (`self.Start`)) false true)
    (`KismetSystemLibrary.Delay` 1.0)
    (set `self.bIsTp` false)))

(fn `UserConstructionScript`
  (`SceneComponent.K2_AddLocalOffset` (`self.Start`) (`self.StartLocation`) false false)
  (`SceneComponent.K2_AddLocalOffset` (`self.End`) (`self.EndLocation`) false false)
  (`SceneComponent.SetRelativeScale3D` (`self.Start`) (`self.StartScale`))
  (`SceneComponent.SetRelativeScale3D` (`self.End`) (`self.EndScale`)))